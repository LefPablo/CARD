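; TEST_BP is a test vehicle pawn Blueprint with basic driving and look controls.
; MoveForward and MoveRight axes feed throttle and steering on its VehicleMovement component, while LookRight and LookUp add controller yaw and pitch.
; BeginPlay calls AttachActorToActor on RootSocket with relative transform rules, but no parent actor is specified.
; The construction script is empty.
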(event EventBeginPlay
  (Transformation|AttachActorToActor self 0 "RootSocket" "KeepRelative" "KeepRelative" "KeepRelative" true))

(event Input|AxisEvents|InputAxisMoveForward
  (params (AxisValue :type Float%20%28single-precision%29))
  (Class|WheeledVehicleMovementComponent|SetThrottleInput (Variables|Default|GetVehicleMovement) AxisValue))

(event Input|AxisEvents|InputAxisMoveRight
  (params (AxisValue :type Float%20%28single-precision%29))
  (Class|WheeledVehicleMovementComponent|SetSteeringInput (Variables|Default|GetVehicleMovement) AxisValue))

(event Input|AxisEvents|InputAxisLookRight
  (params (AxisValue :type Float%20%28single-precision%29))
  (Pawn|Input|AddControllerYawInput AxisValue))

(event Input|AxisEvents|InputAxisLookUp
  (params (AxisValue :type Float%20%28single-precision%29))
  (Pawn|Input|AddControllerPitchInput AxisValue))

(fn ConstructionScript)